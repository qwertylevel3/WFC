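; BP_Luna is a grid-based actor, handled as a block, that turns and moves one direction at a time.
; A bound move event sets orientation, rotates the mesh and asks the zone area to attempt the move from its grid position.
; MoveAnimation plays a timeline that slides the actor along that direction while offsetting the mesh vertically, then snaps it to the target cell's world position.
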(event Custom|EventMoveTo
  (params (Direction :type EWFCOrientation%20Enum :default "E_UP"))
  (bind _self self)
  (Variables|Default|SetOrientation Direction)
  (Utilities|UpdateMeshDirection)
  (bind _area (CallFunction|GetZoneArea))
  (Class|WFCPlayZone|TryMoveBlockbyDirection _area _self (Variables|Default|GetGridPos _self) (Variables|Default|GetOrientation)))

(event EventBeginPlay
  (EventDispatchers|BindEventtoEventMove (delegate Custom|EventMoveTo))
  (Variables|Default|SetLastLocation "0, 0, 0"))

(event EventMoveAnimation
  (params (OriPos :type WFC%20Int%20Vector%20Structure%20%28by%20ref%29) (TargetPos :type WFC%20Int%20Vector%20Structure%20%28by%20ref%29))
  (bind _worldpos (CallFunction|GridPostoWorldPos TargetPos))
  (Variables|Default|SetTargetLocation _worldpos)
  (bind (_direction _z _delta) (Timeline|Timeline_0 PlayFromStart)
    (:Update
      (bind _vec (CallFunction|DirectiontoVector (Variables|Default|GetOrientation)))
      (Transformation|SetRelativeLocation (Variables|Default|GetStaticMesh) (Math|Vector|MakeVector 0.0 0.0 _z) false false)
      (Transformation|SetActorLocation (Math|Vector|MakeVector (.x (+ (Variables|Default|GetLastLocation) (* (* _vec 1.6e+02) _delta))) (.y (+ (Variables|Default|GetLastLocation) (* (* _vec 1.6e+02) _delta))) 0.0) false false))
    (:Finished
      (Transformation|SetActorLocation (Variables|Default|GetTargetLocation) false false)
      (Variables|Default|SetLastLocation (Variables|Default|GetTargetLocation)))))

(fn ConstructionScript)