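; BP_PlayerController is a player controller that turns four directional move inputs into movement of the world area and the Luna pawn.
; Each press calls the matching move function on a BP_WFCArea, then passes a direction enum to BP_Luna's EventMoveTo.
; CheckArea lazily caches the first BP_WFCArea found in the level whenever the stored reference is invalid.
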(event EventBeginPlay)

(event Input|ActionEvents|InputActionMoveForward
  (params (Key :type Key%20Structure))
  (:Pressed
    (CallFunction|CheckArea)
    (Class|WFCArea|MoveForward (Variables|Default|GetArea))
    (bind _asbp_luna (Utilities|Casting|CastToBP_Luna (Game|Player|GetPlayerPawn 0)))
    (Default|EventMoveto _asbp_luna "NewEnumerator0")))

(event Input|ActionEvents|InputActionMoveBack
  (params (Key :type Key%20Structure))
  (:Pressed
    (CallFunction|CheckArea)
    (Class|WFCArea|MoveBack (Variables|Default|GetArea))
    (bind _asbp_luna (Utilities|Casting|CastToBP_Luna (Game|Player|GetPlayerPawn 0)))
    (Default|EventMoveto _asbp_luna "NewEnumerator1")))

(event Input|ActionEvents|InputActionMoveLeft
  (params (Key :type Key%20Structure))
  (:Pressed
    (CallFunction|CheckArea)
    (Class|WFCArea|MoveLeft (Variables|Default|GetArea))
    (bind _asbp_luna (Utilities|Casting|CastToBP_Luna (Game|Player|GetPlayerPawn 0)))
    (Default|EventMoveto _asbp_luna "NewEnumerator2")))

(event Input|ActionEvents|InputActionMoveRight
  (params (Key :type Key%20Structure))
  (:Pressed
    (CallFunction|CheckArea)
    (Class|WFCArea|MoveRight (Variables|Default|GetArea))
    (bind _asbp_luna (Utilities|Casting|CastToBP_Luna (Game|Player|GetPlayerPawn 0)))
    (Default|EventMoveto _asbp_luna "NewEnumerator3")))

(fn ConstructionScript)

(fn CheckArea
  (Utilities|IsValid (Variables|Default|GetArea)
    (:Is%20Valid
      _)
    (:Is%20Not%20Valid
      (bind _outactors (Actor|GetAllActorsOfClass "/Game/BP/BP_WFCArea.BP_WFCArea_C"))
      (Variables|Default|SetArea (Utilities|Array|Get(acopy) _outactors))))
  (return))