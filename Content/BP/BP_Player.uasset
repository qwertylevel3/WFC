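; BP_Player is a player actor that moves in fixed 160-unit grid steps in four directions.
; On BeginPlay it binds to the EventMove dispatcher, whose direction sets the mesh rotation and the next target location.
; A timeline interpolates actor X/Y and drives the mesh's relative Z separately, then snaps to the target on finish.
; The stored grid position starts at world origin and updates only after each step completes.
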(event Custom|EventMovePlayer
  (params (NewParam :type EDirection%20Enum :default "NewEnumerator0"))
  (bind _output_get (Variables|Default|SetOrientation NewParam))
  (Utilities|UpdateMeshDirection)
  ;[1 1 1] set targetlocation
  (bind _vec (CallFunction|DirectiontoVector _output_get))
  (Variables|Default|SetTargetLocation (+ (Variables|Default|GetLastLocation) (* _vec 160)))
  (bind (_direction _z _delta) (Timeline|MoveTimeLine PlayFromStart)
    (:Update
      (bind _vec_2 (CallFunction|DirectiontoVector (Variables|Default|GetOrientation)))
      (Transformation|SetRelativeLocation (Variables|Default|GetStaticMesh) (Math|Vector|MakeVector 0.0 0.0 _z) false false)
      (Transformation|SetActorLocation (Math|Vector|MakeVector (.x (+ (Variables|Default|GetLastLocation) (* (* _vec_2 1.6e+02) _delta))) (.y (+ (Variables|Default|GetLastLocation) (* (* _vec_2 1.6e+02) _delta))) 0.0) false false))
    (:Finished
      (Transformation|SetActorLocation (Variables|Default|GetTargetLocation) false false)
      (Variables|Default|SetLastLocation (Variables|Default|GetTargetLocation)))))

(event EventBeginPlay
  (|CallParentFunction)
  (EventDispatchers|BindEventtoEventMove (delegate Custom|EventMovePlayer))
  (Variables|Default|SetLastLocation "0, 0, 0"))

(event Collision|EventActorBeginOverlap
  (params (OtherActor :type Actor%20Object%20Reference))
  (|CallParentFunction OtherActor) ; 此节点被禁用，将不会被调用。\n从引脚连出引线来编译功能。
)

(event EventTick
  (params (DeltaSeconds :type Float%20%28single-precision%29))
  (|CallParentFunction DeltaSeconds) ; 此节点被禁用，将不会被调用。\n从引脚连出引线来编译功能。
)

(fn ConstructionScript
  (|CallParentFunction))